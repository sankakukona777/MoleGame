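; BP_AttributeSetData is an editor utility data object that exposes an attribute's minimum and maximum clamp settings through separate clamp objects.
; Setup creates two BP_ClampData children and fills each with the type, value and property from AttributeInfo.
; SetupInfo copies both children's values back into the AttributeInfo struct, converting property strings back to names.
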(event `Setup`
  (bind (_attributeinfo_classname _attributeinfo_propertyname _attributeinfo_minclamptype _attributeinfo_minclampvalue _attributeinfo_minclampproperty _attributeinfo_maxclamptype _attributeinfo_maxclampvalue _attributeinfo_maxclampproperty) (break `/KM_GAHelperForBP/DataTables/ST_GEAttribute` (`self.AttributeInfo`)))
  (bind (_attributeinfo_classname_2 _attributeinfo_propertyname_2 _attributeinfo_minclamptype_2 _attributeinfo_minclampvalue_2 _attributeinfo_minclampproperty_2) (break `/KM_GAHelperForBP/DataTables/ST_GEAttribute` (`self.AttributeInfo`)))
  (bind _returnvalue (`|GenericCreateObject` "/KM_GAHelperForBP/EditorUtility/BP_ClampData.BP_ClampData_C" self))
  (set `self.MinClamp` _returnvalue)
  (bind _returnvalue_2 (`|GenericCreateObject` "/KM_GAHelperForBP/EditorUtility/BP_ClampData.BP_ClampData_C" self))
  (set `self.MaxClamp` _returnvalue_2)
  (`/KM_GAHelperForBP/EditorUtility/BP_ClampData.Setup` (`self.MinClamp`) _attributeinfo_minclamptype_2 _attributeinfo_minclampvalue_2 (`KismetStringLibrary.Conv_NameToString` _attributeinfo_minclampproperty_2))
  (`/KM_GAHelperForBP/EditorUtility/BP_ClampData.Setup` (`self.MaxClamp`) _attributeinfo_maxclamptype _attributeinfo_maxclampvalue (`KismetStringLibrary.Conv_NameToString` _attributeinfo_maxclampproperty)))

(event `SetupInfo`
  (bind _minclamp (`self.MinClamp`))
  (bind _maxclamp (`self.MaxClamp`))
  (setmembers `/KM_GAHelperForBP/DataTables/ST_GEAttribute` :`StructRef` (`self.AttributeInfo`) :`MinClampType` (`/KM_GAHelperForBP/EditorUtility/BP_ClampData.ClampType` _minclamp) :`MinClampValue` (`/KM_GAHelperForBP/EditorUtility/BP_ClampData.ClampValue` _minclamp) :`MinClampProperty` (`KismetStringLibrary.Conv_StringToName` (`/KM_GAHelperForBP/EditorUtility/BP_ClampData.ClampProperty` _minclamp)) :`MaxClampType` (`/KM_GAHelperForBP/EditorUtility/BP_ClampData.ClampType` _maxclamp) :`MaxClampValue` (`/KM_GAHelperForBP/EditorUtility/BP_ClampData.ClampValue` _maxclamp) :`MaxClampProperty` (`KismetStringLibrary.Conv_StringToName` (`/KM_GAHelperForBP/EditorUtility/BP_ClampData.ClampProperty` _maxclamp))))