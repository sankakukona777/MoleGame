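; Vertically oscillating lift for the 2D side-scroller that the player can pass through.
; Each Tick it moves by an accelerating speed, flips direction by negating its travel and speed limits, and pauses as speed nears zero, using a re-armed DoOnce.
; The platform mesh ignores collision while the player's capsule overlaps ThroughCollision or during battle events, otherwise blocking.
; DownCollision overlap toggles the character's DownFloorEvent and NotDownFloorEvent.
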(event `self.ReceiveTick`
  (params (DeltaSeconds :type "Float (single-precision)"))
  (if (not (`self.StopFlag`))
    (`self.FlowAbout`)
    (`self.FlowSpeedAbout`)
    (`self.FlowP`))
  (`self.StopEvent`)
  (`self.ThroughP`))

(event `ThroughP`
  (bind `_スラム街用素材_2` (`self.スラム街用素材_2`))
  (bind _as2dside_scroller_character (cast `/Game/2DSideScrollerBP/Blueprints/2DSideScrollerCharacter` (`GameplayStatics.GetPlayerPawn` 0) :!pure true))
  (bind _as2dside_scroller_character_2 (cast `/Game/2DSideScrollerBP/Blueprints/2DSideScrollerCharacter` (`GameplayStatics.GetPlayerPawn` 0) :!pure true))
  ;[1 1 1] すり抜け処理
  (if (`PrimitiveComponent.IsOverlappingComponent` (`self.ThroughCollision`) (`Character.CapsuleComponent` _as2dside_scroller_character_2))
    (`PrimitiveComponent.SetCollisionResponseToAllChannels` `_スラム街用素材_2` "ECR_Ignore" :!label _label)
    (elif (`/Game/2DSideScrollerBP/Blueprints/2DSideScrollerCharacter.BattleEventFlag` _as2dside_scroller_character_2)
      (goto _label)
      (else
        (`PrimitiveComponent.SetCollisionResponseToAllChannels` `_スラム街用素材_2` "ECR_Block"))))
  (if (`PrimitiveComponent.IsOverlappingComponent` (`self.DownCollision`) (`Character.CapsuleComponent` _as2dside_scroller_character))
    (`/Game/2DSideScrollerBP/Blueprints/2DSideScrollerCharacter.DownFloorEvent` _as2dside_scroller_character)
    (else
      (`/Game/2DSideScrollerBP/Blueprints/2DSideScrollerCharacter.NotDownFloorEvent` _as2dside_scroller_character))))

(event `FlowP`
  ;[1 1 1] リフトを動かす処理
  (`self.K2_SetActorLocation` (`KismetMathLibrary.MakeVector` (.x (`self.K2_GetActorLocation`)) (.y (`self.K2_GetActorLocation`)) (+ (.z (`self.K2_GetActorLocation`)) (`self.FlowSpeed`))))
  (set `self.FlowHeightSum` (+ (`self.FlowHeightSum`) (`self.FlowSpeed`))))

(event `FlowAbout`
  ;[1 1 1] 上下の切替
  (if (`self.FlowDirection`)
    (if (> (`self.FlowHeightSum`) (`self.FlowHeightMAX`))
      (set `self.FlowDirection` false)
      (set `self.FlowHeightMAX` (* (`self.FlowHeightMAX`) -1.0) :!label _label_2)
      (set `self.FlowHeightSum` 0.0)
      (set `self.FlowSpeedMAX` (* (`self.FlowSpeedMAX`) -1.0)))
    (elif (< (`self.FlowHeightSum`) (`self.FlowHeightMAX`))
      (set `self.FlowDirection` true)
      (goto _label_2))))

(event `FlowSpeedAbout`
  ;[1 1 1] リフトスピードの処理
  (if (`self.FlowDirection`)
    (if (< (`self.FlowSpeed`) (`self.FlowSpeedMAX`))
      (set `self.FlowSpeed` (+ (`self.FlowSpeed`) (`self.FlowAddSpeed`)))
      (set `self.StopFlag2` true))
    (elif (> (`self.FlowSpeed`) (`self.FlowSpeedMAX`))
      (set `self.FlowSpeed` (- (`self.FlowSpeed`) (`self.FlowAddSpeed`)))
      (set `self.StopFlag2` true))))

(event `StopEvent`
  ;[1 1 1] 止まる処理
  (if (`KismetMathLibrary.NearlyEqual_FloatFloat` (`self.FlowSpeed`) 0.0 0.5)
    (`/Engine/EditorBlueprintResources/StandardMacros.DoOnce` false :!label _label_3
      (:`Completed`
        (set `self.StopFlag` true)
        (`KismetSystemLibrary.Delay` (`self.StopTime`))
        (set `self.StopFlag` false)))
    (elif (`self.StopFlag2`)
      (set `self.StopFlag2` false)
      (goto _label_3 :!via `Reset`))))

(fn `UserConstructionScript`)