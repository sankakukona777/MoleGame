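; BP_MudCore_3 is a diggable mud core object for a 2D side-scroller that breaks once its life runs out.
; Each Tick it tests overlap with the player's collision for the active dig direction, decrementing life and triggering sound and delayed force feedback.
; While alive, its flipbook nudges up and down on certain frames.
; At zero life it increments NoPlayGameMode's CrashCount, destroys its main components and reveals a break flipbook.
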(event `self.ReceiveBeginPlay`
  (`SceneComponent.SetHiddenInGame` (`self.PaperFlipbook1`) true false))

(event `self.ReceiveTick`
  (params (DeltaSeconds :type "Float (single-precision)"))
  (`self.DoBreakEvent`)
  (if (> (`self.ObjectLife`) 0)
    (`self.UpdateAnimation`)))

(event `DoBreakEvent`
  (bind _objectlife (`self.ObjectLife`))
  (bind _digactioncollision (`self.DigActionCollision`))
  (bind _as2dside_scroller_character (cast `/Game/2DSideScrollerBP/Blueprints/2DSideScrollerCharacter` (`GameplayStatics.GetPlayerPawn` 0) :!pure true))
  (if (> (`self.ObjectLife`) 0)
    ;[1 1 1] 接触イベントをプレイヤー&掘るアクション中に限定
    (if (`/Game/2DSideScrollerBP/Blueprints/2DSideScrollerCharacter.DigActionN` _as2dside_scroller_character)
      (if (`PrimitiveComponent.IsOverlappingComponent` _digactioncollision (`/Game/2DSideScrollerBP/Blueprints/2DSideScrollerCharacter.DigActionCollision` _as2dside_scroller_character))
        ;[1 1 1] オブジェクトのライフを減らす
        (set `self.ObjectLife` (- _objectlife 1) :!label _label)
        (if (== _objectlife 0)
          (`self.CrashCount`)
          (`self.Destroy Object`)
          (`/Game/2DSideScrollerBP/Blueprints/2DSideScrollerCharacter.SoundMusic_MudCore` (cast `/Game/2DSideScrollerBP/Blueprints/2DSideScrollerCharacter` (`GameplayStatics.GetPlayerPawn` 0) :!pure true) :!label _label_2)
          (`KismetSystemLibrary.Delay` 0.3)
          (`PlayerController.K2_ClientPlayForceFeedback` (`GameplayStatics.GetPlayerController` 0) "/Game/AdditionalContents/FeedbackEffect/MudCoreFeedbackEffect.MudCoreFeedbackEffect" "None" false false false)
          (elif (> _objectlife 0)
            (`self.Damage Effect`)
            (goto _label_2))))
      (elif (`/Game/2DSideScrollerBP/Blueprints/2DSideScrollerCharacter.DigActionUP` _as2dside_scroller_character)
        (if (`PrimitiveComponent.IsOverlappingComponent` _digactioncollision (`/Game/2DSideScrollerBP/Blueprints/2DSideScrollerCharacter.DigActionCollisionUP` _as2dside_scroller_character))
          (goto _label))
        (elif (`/Game/2DSideScrollerBP/Blueprints/2DSideScrollerCharacter.DigActionDown` _as2dside_scroller_character)
          (if (`PrimitiveComponent.IsOverlappingComponent` _digactioncollision (`/Game/2DSideScrollerBP/Blueprints/2DSideScrollerCharacter.DigActionCollisionDOWN` _as2dside_scroller_character))
            (goto _label)))))))

(event `UpdateAnimation`
  (bind _paperflipbook (`self.PaperFlipbook`))
  (bind _returnvalue (`PaperFlipbookComponent.GetPlaybackPositionInFrames` (`self.PaperFlipbook`)))
  (bind _x (.x (`SceneComponent.K2_GetComponentLocation` _paperflipbook)))
  (bind _y (.y (`SceneComponent.K2_GetComponentLocation` _paperflipbook)))
  (bind _z (.z (`SceneComponent.K2_GetComponentLocation` _paperflipbook)))
  (if (> _returnvalue 22)
    (if (< _returnvalue 26)
      (`SceneComponent.K2_SetWorldLocation` _paperflipbook (`KismetMathLibrary.MakeVector` _x _y (+ _z 0.3)) false false)
      (elif (< _returnvalue 29)
        (`SceneComponent.K2_SetWorldLocation` _paperflipbook (`KismetMathLibrary.MakeVector` _x _y (- _z 0.3)) false false)))))

(event `Damage Effect`)

(event `Destroy Object`
  (bind _paperflipbook1 (`self.PaperFlipbook1`))
  ;[1 1 1] Shape_Cube(見た目用)の消去
  (`ActorComponent.K2_DestroyComponent` (`self.MainCollision`))
  (`ActorComponent.K2_DestroyComponent` (`self.PaperFlipbook`))
  (`ActorComponent.K2_DestroyComponent` (`self.DigActionCollision`))
  ;[1 1 1] 壊れアニメーションを出現
  (`SceneComponent.SetHiddenInGame` _paperflipbook1 false false)
  (`PaperFlipbookComponent.SetPlaybackPositionInFrames` _paperflipbook1 0 false)
  (`KismetSystemLibrary.Delay` 0.7)
  (`PaperFlipbookComponent.SetPlayRate` _paperflipbook1 0.0))

(event `CrashCount`
  ;[1 1 1] NoPlayGameModeのクラッシュカウントにプラスする
  (bind _asno_play_game_mode (cast `/Game/AdditionalContents/GameMode/NoPlayGameMode` (`GameplayStatics.GetGameMode`)))
  (set `/Game/AdditionalContents/GameMode/NoPlayGameMode.CrashCount` (+ (`/Game/AdditionalContents/GameMode/NoPlayGameMode.CrashCount` _asno_play_game_mode) 1) _asno_play_game_mode))

(fn `UserConstructionScript`)