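; Side-scroller camera actor that becomes the view target and follows the player within bounds set by four edge actors.
; Each Tick runs the follow logic, three frame-counted hit-stop shakes (random, vertical, sideways) and the battle zoom, all by moving the actor.
; Events set shake flags and parameters.
; BattleStart halts following, offsets toward the player's facing and steps in along Y; BattleEnd snaps to bounds and lets the zoom undo itself.
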(event `self.ReceiveBeginPlay`
  (`PlayerController.SetViewTargetWithBlend` (`GameplayStatics.GetPlayerController` 0) self 0.0 "VTBlend_Linear" 0.0 false))

(event `BattleStartEvent`)

(event `self.ReceiveTick`
  (params (DeltaSeconds :type "Float (single-precision)"))
  (if (not (`self.BattleEventFlag_Zoom`))
    (`self.CameraFlow`))
  (`self.HitStopFlow_Random`)
  (`self.HitStopFlow_Vertical`)
  (`self.HitStopFlow_Beside`)
  (`self.BattleEvent_Zoom`))

(event `CameraFlow`
  (bind _returnvalue (`self.K2_GetActorLocation` (`GameplayStatics.GetPlayerPawn` 0)))
  (bind _returnvalue_2 (`self.K2_GetActorLocation` self))
  (bind _x (.x _returnvalue))
  (bind _z (.z _returnvalue))
  (bind _y (.y _returnvalue_2))
  (bind _returnvalue_3 (< (.z (`self.K2_GetActorLocation` (`self.DownEnd`))) _z))
  (bind _returnvalue_4 (> (.z (`self.K2_GetActorLocation` (`self.UpEnd`))) _z))
  ;[1 1 1] プレイヤーを追う処理
  (if (< (.x (`self.K2_GetActorLocation` (`self.LeftEnd`))) _x)
    (if (> (.x (`self.K2_GetActorLocation` (`self.RightEnd`))) _x)
      (if _returnvalue_4
        (if _returnvalue_3
          (`self.K2_SetActorLocation` (+ _returnvalue (0.0 700.0 0.0)) true)
          (else
            (`self.K2_SetActorLocation` (`KismetMathLibrary.MakeVector` (.x _returnvalue) _y (.z _returnvalue_2)) true :!label _label)))
        (else
          (goto _label)))
      (else
        (if _returnvalue_4 :!label _label_2
          (if _returnvalue_3
            (`self.K2_SetActorLocation` (`KismetMathLibrary.MakeVector` (.x _returnvalue_2) _y (.z _returnvalue)) true)
            (else
              (`self.K2_SetActorLocation` _returnvalue_2 true :!label _label_3)))
          (else
            (goto _label_3)))))
    (else
      (goto _label_2))))

(event `BattleEvent_Zoom`
  (bind _hitstopcount (`self.HitStopCount`))
  (bind _x (.x (`self.K2_GetActorLocation` self)))
  (bind _y (.y (`self.K2_GetActorLocation` self)))
  (bind _z (.z (`self.K2_GetActorLocation` self)))
  ;[1 1 1] ズームの処理
  (if (`self.BattleEventFlag_Zoom`)
    (set `self.HitStopCount` (+ _hitstopcount 1))
    (if (not (> _hitstopcount (`self.ShakeTime_SomeShakeTime`)))
      (`self.K2_SetActorLocation` (`KismetMathLibrary.MakeVector` _x (- _y (`self.ZoomValue`)) _z) true)
      (set `self.ZoomTotal` (+ (`self.ZoomTotal`) (`self.ZoomValue`))))
    (else
      (`self.K2_SetActorLocation` (`KismetMathLibrary.MakeVector` _x (+ _y (`self.ZoomTotal`)) _z) true)
      (set `self.ZoomTotal` 0.0))))

(event `HitStopFlow_Beside`
  (bind _shakevalue (`self.ShakeValue`))
  (bind _hitstopcount (`self.HitStopCount`))
  (bind _x (.x (`self.K2_GetActorLocation` self)))
  (bind _y (.y (`self.K2_GetActorLocation` self)))
  (bind _z (.z (`self.K2_GetActorLocation` self)))
  (bind _returnvalue (/ (mod _hitstopcount (`self.ShakeTime_OneShakeTime`)) (`self.ShakeTime_Interal`)))
  ;[1 1 1] 揺れの処理(横)
  (if (`self.HitStopFlag_Beside`)
    (set `self.HitStopCount` (+ _hitstopcount 1))
    (if (> _hitstopcount (`self.ShakeTime_SomeShakeTime`))
      (set `self.HitStopCount` 0)
      (set `self.HitStopFlag_Beside` false)
      (elif (`self.ShakeDirectioRight`)
        (switch `int` _returnvalue
          (:`0`
            (`self.K2_SetActorLocation` (`KismetMathLibrary.MakeVector` (+ _x _shakevalue) _y _z) true :!label _label_4))
          (:`1`
            (`self.K2_SetActorLocation` (`KismetMathLibrary.MakeVector` (- _x _shakevalue) _y _z) true :!label _label_5)))
        (else
          (switch `int` _returnvalue
            (:`0`
              (goto _label_5))
            (:`1`
              (goto _label_4))))))))

(event `HitStopFlow_Random`
  (bind _hitstopcount (`self.HitStopCount`))
  (bind _shakevalue (`self.ShakeValue`))
  (bind _x (.x (`self.K2_GetActorLocation` self)))
  (bind _y (.y (`self.K2_GetActorLocation` self)))
  (bind _z (.z (`self.K2_GetActorLocation` self)))
  (bind _returnvalue (- _x _shakevalue))
  (bind _returnvalue_2 (- _z _shakevalue))
  (bind _returnvalue_3 (+ _x _shakevalue))
  (bind _returnvalue_4 (+ _z _shakevalue))
  ;[1 1 1] 揺れの処理(ランダム)
  (if (`self.HitStopFlag_Random`)
    (set `self.HitStopCount` (+ _hitstopcount 1))
    (if (> _hitstopcount (`self.ShakeTime_SomeShakeTime`))
      (set `self.HitStopCount` 0)
      (set `self.HitStopFlag_Random` false)
      (else
        (switch `int` (/ (mod _hitstopcount (`self.ShakeTime_OneShakeTime`)) (`self.ShakeTime_Interal`))
          (:`0`
            (`self.K2_SetActorLocation` (`KismetMathLibrary.MakeVector` _returnvalue_3 _y _returnvalue_4) true))
          (:`1`
            (`self.K2_SetActorLocation` (`KismetMathLibrary.MakeVector` _returnvalue_3 _y _returnvalue_2) true))
          (:`2`
            (`self.K2_SetActorLocation` (`KismetMathLibrary.MakeVector` _returnvalue _y _returnvalue_4) true))
          (:`3`
            (`self.K2_SetActorLocation` (`KismetMathLibrary.MakeVector` _returnvalue _y _returnvalue_2) true)))))))

(event `HitStopFlow_Vertical`
  (bind _hitstopcount (`self.HitStopCount`))
  (bind _shakevalue (`self.ShakeValue`))
  (bind _x (.x (`self.K2_GetActorLocation` self)))
  (bind _y (.y (`self.K2_GetActorLocation` self)))
  (bind _z (.z (`self.K2_GetActorLocation` self)))
  ;[1 1 1] 揺れの処理(縦)
  (if (`self.HitStopFlag_Vertical`)
    (set `self.HitStopCount` (+ _hitstopcount 1))
    (if (> _hitstopcount (`self.ShakeTime_SomeShakeTime`))
      (set `self.HitStopCount` 0)
      (set `self.HitStopFlag_Vertical` false)
      (else
        (switch `int` (/ (mod _hitstopcount (`self.ShakeTime_OneShakeTime`)) (`self.ShakeTime_Interal`))
          (:`0`
            (`self.K2_SetActorLocation` (`KismetMathLibrary.MakeVector` _x _y (+ _z _shakevalue)) true))
          (:`1`
            (`self.K2_SetActorLocation` (`KismetMathLibrary.MakeVector` _x _y (- _z _shakevalue)) true)))))))

(event `HitStopEvent_Core`
  ;[1 1 1] HitStop&揺れ関連(コア)
  (set `self.HitStopFlag_Random` true) ; 揺れの種類(縦・横・ランダム)
  (set `self.ShakeValue` 30.0) ; 揺れの大きさ
  (set `self.ShakeTime_SomeShakeTime` 6) ; 揺れの全体時間
  (set `self.ShakeTime_OneShakeTime` 4) ; 1処理の時間
  (set `self.ShakeTime_Interal` 1) ; 1揺れの感覚
)

(event `HitStopEvent_Enemy_Right`
  ;[1 1 1] HitStop&揺れ関連(敵)
  (set `self.HitStopFlag_Vertical` true)
  (set `self.HitStopFlag_Random` false)
  (set `self.ShakeValue` 500.0)
  (set `self.ShakeTime_SomeShakeTime` 6)
  (set `self.ShakeTime_OneShakeTime` 6)
  (set `self.ShakeTime_Interal` 3)
  (set `self.HitStopCount` 0))

(event `BattleStart`
  (bind _returnvalue (`GameplayStatics.GetPlayerPawn` 0))
  (bind _y (.y (`self.K2_GetActorLocation` self)))
  (bind _x (.x (`self.K2_GetActorLocation` _returnvalue)))
  (bind _z (.z (`self.K2_GetActorLocation` _returnvalue)))
  ;[1 1 1] 戦闘時
  (set `self.BattleEventFlag_Zoom` true)
  (set `self.ShakeTime_SomeShakeTime` 21)
  (set `self.ZoomValue` 15.0)
  (if (`/Game/2DSideScrollerBP/Blueprints/2DSideScrollerCharacter.bisMovingRight` (cast `/Game/2DSideScrollerBP/Blueprints/2DSideScrollerCharacter` _returnvalue :!pure true))
    (`self.K2_SetActorLocation` (`KismetMathLibrary.MakeVector` (+ _x 300.0) _y _z) true)
    (else
      (`self.K2_SetActorLocation` (`KismetMathLibrary.MakeVector` (- _x 300.0) _y _z) true))))

(event `BattleEnd`
  (bind _returnvalue (`self.K2_GetActorLocation` self))
  (bind _returnvalue_2 (`self.K2_GetActorLocation` (`GameplayStatics.GetPlayerPawn` 0)))
  (bind _z (.z (`self.K2_GetActorLocation` (`self.UpEnd`))))
  (bind _x (.x _returnvalue_2))
  (bind _y (.y _returnvalue))
  (bind _x_2 (.x (`self.K2_GetActorLocation` (`self.RightEnd`))))
  (bind _x_3 (.x _returnvalue_2))
  (bind _z_2 (.z _returnvalue_2))
  (bind _z_3 (.z (`self.K2_GetActorLocation` (`self.DownEnd`))))
  (bind _z_4 (.z _returnvalue_2))
  (bind _x_4 (.x (`self.K2_GetActorLocation` (`self.LeftEnd`))))
  (bind _returnvalue_3 (< _z_3 _z_2))
  (bind _returnvalue_4 (> _z _z_2))
  ;[1 1 1] 戦闘時
  (set `self.HitStopCount` 0)
  (set `self.BattleEventFlag_Zoom` false)
  (if (< _x_4 _x_3)
    (if (> _x_2 _x_3)
      (if _returnvalue_4
        (if _returnvalue_3
          (`self.K2_SetActorLocation` _returnvalue true)
          (else
            (`self.K2_SetActorLocation` (`KismetMathLibrary.MakeVector` _x _y _z_3) true)))
        (else
          (`self.K2_SetActorLocation` (`KismetMathLibrary.MakeVector` _x _y _z) true)))
      (elif _returnvalue_4
        (if _returnvalue_3
          (`self.K2_SetActorLocation` (`KismetMathLibrary.MakeVector` _x_2 _y _z_4) true)
          (else
            (`self.K2_SetActorLocation` (`KismetMathLibrary.MakeVector` _x_2 _y _z_3) true)))
        (else
          (`self.K2_SetActorLocation` (`KismetMathLibrary.MakeVector` _x_2 _y _z) true))))
    (elif _returnvalue_4
      (if _returnvalue_3
        (`self.K2_SetActorLocation` (`KismetMathLibrary.MakeVector` _x_4 _y _z_4) true)
        (else
          (`self.K2_SetActorLocation` (`KismetMathLibrary.MakeVector` _x_4 _y _z_3) true)))
      (else
        (`self.K2_SetActorLocation` (`KismetMathLibrary.MakeVector` _x_4 _y _z) true)))))

(event `FinishEvent_VendingMachine`
  ;[1 1 1] HitStop&揺れ関連(敵)
  (set `self.HitStopFlag_Random` true)
  (set `self.ShakeValue` 30.0))

(fn `UserConstructionScript`)