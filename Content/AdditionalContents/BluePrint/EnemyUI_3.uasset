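; Side-scroller enemy that stays hidden while overlapping the mud core's dig collision, then appears and starts a quick-time-event battle with the player.
; Tick drives every stage: flags gate a manual X/Z chase of the player and signal the character and camera.
; Random-key QTE successes remove life and trigger a hand-coded arc knockback, re-arming the next QTE.
; At zero life it ends the battle and destroys itself after a delay.
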(event `self.ReceiveBeginPlay`
  (`SceneComponent.SetHiddenInGame` (`self.Widget`) true false)
  (`SceneComponent.SetHiddenInGame` (`self.PaperSprite`) true false))

(event `self.ReceiveTick`
  (params (DeltaSeconds :type "Float (single-precision)"))
  (`self.AppearEvent`)
  (`self.BattleStartEvent`)
  (`self.BlowAwayEvent`)
  (`self.DestroyEvent`))

(event `AppearEvent`
  (bind _papersprite (`self.PaperSprite`))
  (bind _enemyspeed (`self.EnemySpeed`))
  (bind _widget (`self.Widget`))
  (bind _enemylashdistance_z (`self.EnemyLashDistance_Z`))
  (bind _enemylashdistance_x (`self.EnemyLashDistance_X`))
  (bind _returnvalue (`self.K2_GetActorLocation` (`GameplayStatics.GetPlayerPawn` 0)))
  (bind _returnvalue_2 (`self.K2_GetActorLocation` self))
  (bind _returnvalue_3 (+ _enemylashdistance_x _enemylashdistance_z))
  (bind _x (.x _returnvalue_2))
  (bind _y (.y _returnvalue_2))
  (bind _z (.z _returnvalue_2))
  (bind _x_2 (.x _returnvalue_2))
  (bind _z_2 (.z _returnvalue_2))
  (bind _x_3 (.x _returnvalue))
  (bind _z_3 (.z _returnvalue))
  (bind _returnvalue_4 (> (.z _returnvalue_2) (.z _returnvalue)))
  (bind _returnvalue_5 (- _z_2 _z_3))
  (bind _returnvalue_6 (- _z_3 _z_2))
  (bind _returnvalue_7 (* (/ _enemylashdistance_x _returnvalue_3) _enemyspeed))
  (bind _returnvalue_8 (* (/ _enemylashdistance_z _returnvalue_3) _enemyspeed))
  (bind _returnvalue_9 (- _x _returnvalue_7))
  (bind _returnvalue_10 (- _z _returnvalue_8))
  (bind _returnvalue_11 (+ _x _returnvalue_7))
  (bind _returnvalue_12 (+ _z _returnvalue_8))
  (bind _outactors (`GameplayStatics.GetAllActorsOfClass` "/Game/Objects/BP_MudCore_3.BP_MudCore_3_C"))
  (if (`PrimitiveComponent.IsOverlappingComponent` (`self.Sphere`) (`/Game/Objects/BP_MudCore_3.DigActionCollision` (`|GetArrayItem` _outactors)))
    (`SceneComponent.SetHiddenInGame` _widget true false)
    (`SceneComponent.SetHiddenInGame` _papersprite true false)
    (set `self.Appearance_Vertical` 10.0)
    (else
      (`SceneComponent.SetHiddenInGame` _widget false false)
      (`SceneComponent.SetHiddenInGame` _papersprite false false)
      (if (`self.BattleFlag`)
        (if (`self.BattleFlag2`)
          (if (not (`self.BlowFlag`))
            ;[1 1 1] 追尾の処理
            (if (> (.x _returnvalue_2) (.x _returnvalue))
              (set `self.EnemyLashDistance_X` (- _x_2 _x_3))
              (if _returnvalue_4
                (set `self.EnemyLashDistance_Z` _returnvalue_5)
                (`self.K2_SetActorLocation` (`KismetMathLibrary.MakeVector` _returnvalue_9 _y _returnvalue_10))
                (else
                  (set `self.EnemyLashDistance_Z` _returnvalue_6)
                  (`self.K2_SetActorLocation` (`KismetMathLibrary.MakeVector` _returnvalue_9 _y _returnvalue_12))))
              (else
                (set `self.EnemyLashDistance_X` (- _x_3 _x_2))
                (if _returnvalue_4
                  (set `self.EnemyLashDistance_Z` _returnvalue_5)
                  (`self.K2_SetActorLocation` (`KismetMathLibrary.MakeVector` _returnvalue_11 _y _returnvalue_10))
                  (else
                    (set `self.EnemyLashDistance_Z` _returnvalue_6)
                    (`self.K2_SetActorLocation` (`KismetMathLibrary.MakeVector` _returnvalue_11 _y _returnvalue_12))))))
            (`/Engine/EditorBlueprintResources/StandardMacros.DoOnce` false
              (:`Completed`
                (bind _outactors_2 (`GameplayStatics.GetAllActorsOfClass` "/Game/Objects/カメラ関係/BP_CharacterCamera.BP_CharacterCamera_C"))
                (`/Game/Objects/カメラ関係/BP_CharacterCamera.BattleStart` (`|GetArrayItem` _outactors_2))))))
        (else
          (set `self.BattleFlag` true)
          (set `self.Appearance_Beside` 1.0)
          (set `self.AppearanceLimit` -3.0)
          (set `self.Appearance_Vertical` 10.0)
          (`KismetSystemLibrary.Delay` 1.0)
          (set `self.BattleFlag2` true))))))

(event `BattleStartEvent`
  (bind _as2dside_scroller_character (cast `/Game/2DSideScrollerBP/Blueprints/2DSideScrollerCharacter` (`GameplayStatics.GetPlayerPawn` 0) :!pure true))
  (bind _eventwidget (make `/Game/2DSideScrollerBP/QTE/EventWidget` (make `Anchors` (0.5 0.5) (0.5 0.5))))
  ;[1 1 1] 戦闘処理
  (if (`self.BattleFlag`)
    (if (`self.BattleFlag2`)
      (if (not (`self.BlowFlag`))
        (`/Engine/EditorBlueprintResources/StandardMacros.DoOnce` false :!label _label
          (:`Completed`
            (if (not (== (`self.EnemyLife`) 0))
              (switch `int` (`KismetMathLibrary.RandomInteger` 3)
                (:`0`
                  (`/Game/2DSideScrollerBP/QTE/QTE_Library.StartQTE` _as2dside_scroller_character "J" _eventwidget 0.7 0.1
                    (:`Sucsess`
                      _)))
                (:`1`
                  (`/Game/2DSideScrollerBP/QTE/QTE_Library.StartQTE` _as2dside_scroller_character "N" _eventwidget 0.7 0.1
                    (:`Sucsess`
                      _)))
                (:`2`
                  (`/Game/2DSideScrollerBP/QTE/QTE_Library.StartQTE` _as2dside_scroller_character "B" _eventwidget 0.7 0.1
                    (:`Sucsess`
                      _))))
              (set `self.EnemyLife` (- (`self.EnemyLife`) 1))
              (set `self.DamageFlag` true)
              (set `self.BlowFlag` true)
              (set `self.AppearanceLimit` -5.0)
              (set `self.Appearance_Vertical` 5.0)
              (set `self.Appearance_Beside` 4.0)
              (goto _label :!via `Reset`)))))
      (else
        (`/Engine/EditorBlueprintResources/StandardMacros.DoOnce` false
          (:`Completed`
            (`/Game/2DSideScrollerBP/Blueprints/2DSideScrollerCharacter.BattleEventStart` _as2dside_scroller_character)))))))

(event `BlowAwayEvent`
  (bind _appearance_vertical (`self.Appearance_Vertical`))
  (bind _damageflag (`self.DamageFlag`))
  (bind _appearance_beside (`self.Appearance_Beside`))
  (bind _x (.x (`self.K2_GetActorLocation` self)))
  ;[1 1 1] 吹っ飛び処理(出現)
  (if (`self.BlowFlag`)
    (if (< (.x (`self.K2_GetActorLocation` (`GameplayStatics.GetPlayerPawn` 0))) _x)
      (set `self.EnemyDirection` true)
      (if _damageflag
        (if (not (> _appearance_beside 0.0)) :!label _label_2
          (set `self.Appearance_Beside` (* -1 _appearance_beside) :!label _label_3))
        (else
          (if (< _appearance_beside 0.0) :!label _label_4
            _
            (else
              (goto _label_3)))))
      (else
        (set `self.EnemyDirection` false)
        (if _damageflag
          (goto _label_4)
          (else
            (goto _label_2)))))
    (if (< _appearance_vertical (`self.AppearanceLimit`))
      (set `self.BlowFlag` false)
      (set `self.DamageFlag` false)
      (else
        (set `self.Appearance_Vertical` (- _appearance_vertical 0.2))
        (`self.K2_SetActorLocation` (`KismetMathLibrary.MakeVector` (+ _appearance_beside _x) (.y (`self.K2_GetActorLocation` self)) (+ (.z (`self.K2_GetActorLocation` self)) _appearance_vertical)))))))

(event `DestroyEvent`
  ;[1 1 1] 死亡処理
  (if (== (`self.EnemyLife`) 0)
    (`/Game/2DSideScrollerBP/Blueprints/2DSideScrollerCharacter.BattleEventEnd` (cast `/Game/2DSideScrollerBP/Blueprints/2DSideScrollerCharacter` (`GameplayStatics.GetPlayerPawn` 0) :!pure true))
    (`KismetSystemLibrary.Delay` 0.7)
    (`self.K2_DestroyActor`)))

(fn `UserConstructionScript`)