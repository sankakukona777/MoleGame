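; BP_CharacterCamera is a side-view camera actor that becomes the first player's view target on BeginPlay and follows the pawn.
; Each Tick, while the pawn's X lies between the LeftEnd and RightEnd actors, it moves to the pawn's location plus a fixed Y offset.
; Outside that range it holds its X and Y and tracks only the pawn's height, using swept moves in both cases.
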(event `self.ReceiveBeginPlay`
  (`PlayerController.SetViewTargetWithBlend` (`GameplayStatics.GetPlayerController` 0) self 0.0 "VTBlend_Linear" 0.0 false))

(event `self.ReceiveTick`
  (params (DeltaSeconds :type "Float (single-precision)"))
  (bind _returnvalue (`self.K2_GetActorLocation` (`GameplayStatics.GetPlayerPawn` 0)))
  (bind _x (.x (`self.K2_GetActorLocation` (`GameplayStatics.GetPlayerPawn` 0))))
  ;[1 1 1] プレイヤーを追う処理
  (if (< (.x (`self.K2_GetActorLocation` (`self.LeftEnd`))) _x)
    (if (> (.x (`self.K2_GetActorLocation` (`self.RightEnd`))) _x)
      (`self.K2_SetActorLocation` (+ _returnvalue (0.0 700.0 0.0)) true)
      (else
        (`self.K2_SetActorLocation` (`KismetMathLibrary.MakeVector` (.x (`self.K2_GetActorLocation` self)) (.y (`self.K2_GetActorLocation` self)) (.z _returnvalue)) true :!label _label)))
    (else
      (goto _label))))

(fn `UserConstructionScript`)