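; BP_MudCore is a destructible block that the 2DSideScrollerCharacter breaks by digging.
; Tick polls the three directional dig flags and hitbox overlaps, removing one ObjectLife per overlapping tick.
; Surviving hits trigger camera hit stop and re-fracture one of two destructible meshes, alternating by life parity.
; The final hit increments NoPlayGameMode's CrashCount, shatters both meshes with gravity and physics-only collision, and drives their opacity by timeline.
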(event `self.ReceiveTick`
  (params (DeltaSeconds :type "Float (single-precision)"))
  (bind _objectlife (`self.ObjectLife`))
  (bind _digactioncollision (`self.DigActionCollision`))
  (bind _as2dside_scroller_character (cast `/Game/2DSideScrollerBP/Blueprints/2DSideScrollerCharacter` (`GameplayStatics.GetPlayerPawn` 0) :!pure true))
  (if (> (`self.ObjectLife`) 0)
    ;[1 1 1] 接触イベントをプレイヤー&掘るアクション中に限定
    (if (`/Game/2DSideScrollerBP/Blueprints/2DSideScrollerCharacter.DigActionN` _as2dside_scroller_character)
      (if (`PrimitiveComponent.IsOverlappingComponent` _digactioncollision (`/Game/2DSideScrollerBP/Blueprints/2DSideScrollerCharacter.DigActionCollision` _as2dside_scroller_character))
        ;[1 1 1] オブジェクトのライフを減らす
        (set `self.ObjectLife` (- _objectlife 1) :!label _label)
        (if (== _objectlife 0)
          (`self.CrashCount`)
          (`self.Destroy Object`)
          (elif (> _objectlife 0)
            (`self.Damage Effect`)
            (bind _outactors (`GameplayStatics.GetAllActorsOfClass` "/Game/AdditionalContents/BluePrint/Camera/BP_CharacterCamera.BP_CharacterCamera_C"))
            (`/Game/AdditionalContents/BluePrint/Camera/BP_CharacterCamera.HitStopEvent_Core` (`|GetArrayItem` _outactors)))))
      (elif (`/Game/2DSideScrollerBP/Blueprints/2DSideScrollerCharacter.DigActionUP` _as2dside_scroller_character)
        (if (`PrimitiveComponent.IsOverlappingComponent` _digactioncollision (`/Game/2DSideScrollerBP/Blueprints/2DSideScrollerCharacter.DigActionCollisionUP` _as2dside_scroller_character))
          (goto _label))
        (elif (`/Game/2DSideScrollerBP/Blueprints/2DSideScrollerCharacter.DigActionDown` _as2dside_scroller_character)
          (if (`PrimitiveComponent.IsOverlappingComponent` _digactioncollision (`/Game/2DSideScrollerBP/Blueprints/2DSideScrollerCharacter.DigActionCollisionDOWN` _as2dside_scroller_character))
            (goto _label)))))))

(event `Damage Effect`
  (bind _shape_cube_dm_core2 (`self.Shape_Cube_DM_Core2`))
  (bind _shape_cube_dm_core (`self.Shape_Cube_DM_Core`))
  (bind _returnvalue (`SceneComponent.K2_GetComponentLocation` _shape_cube_dm_core))
  (bind _returnvalue_2 (`SceneComponent.K2_GetComponentLocation` _shape_cube_dm_core2))
  ;[1 1 1] 攻撃ごとに発生するエフェクト
  (if (== (mod (`self.ObjectLife`) 2) 1)
    (`DestructibleComponent.SetDestructibleMesh` _shape_cube_dm_core "/Game/Materials/Shape_Cube_DM.Shape_Cube_DM")
    (`DestructibleComponent.ApplyDamage` _shape_cube_dm_core 500.0 _returnvalue _returnvalue 3000.0)
    (else
      (`DestructibleComponent.SetDestructibleMesh` _shape_cube_dm_core2 "/Game/Materials/Shape_Cube_DM.Shape_Cube_DM")
      (`DestructibleComponent.ApplyDamage` _shape_cube_dm_core2 500.0 _returnvalue_2 _returnvalue_2 3000.0))))

(event `Destroy Object`
  (bind _shape_cube_dm_core (`self.Shape_Cube_DM_Core`))
  (bind _shape_cube_dm_core2 (`self.Shape_Cube_DM_Core2`))
  (bind _returnvalue (`SceneComponent.K2_GetComponentLocation` _shape_cube_dm_core2))
  (bind _returnvalue_2 (`SceneComponent.K2_GetComponentLocation` _shape_cube_dm_core))
  ;[1 1 1] ShapeCube_DMにダメージ
  (`DestructibleComponent.ApplyDamage` _shape_cube_dm_core 500.0 _returnvalue_2 _returnvalue_2 5000.0)
  (`DestructibleComponent.ApplyDamage` _shape_cube_dm_core2 500.0 _returnvalue _returnvalue 5000.0)
  ;[1 1 1] Shape_Cube(見た目用)の消去
  (`ActorComponent.K2_DestroyComponent` (`self.Shape_Cube_DM_App`))
  (`ActorComponent.K2_DestroyComponent` (`self.DigActionCollision`))
  ;[1 1 1] 重力付与
  (`PrimitiveComponent.SetEnableGravity` (`self.Shape_Cube_DM_Core`) true)
  (`PrimitiveComponent.SetEnableGravity` (`self.Shape_Cube_DM_Core2`) true)
  ;[1 1 1] 0.1秒後にコリジョンをPhysics Onlyにする
  (`KismetSystemLibrary.Delay` 0.1)
  (`PrimitiveComponent.SetCollisionEnabled` (`self.Shape_Cube_DM_Core`) "PhysicsOnly")
  (`PrimitiveComponent.SetCollisionEnabled` (`self.Shape_Cube_DM_Core2`) "PhysicsOnly")
  (bind _returnvalue_3 (`PrimitiveComponent.CreateDynamicMaterialInstance` (`self.Shape_Cube_DM_Core`) 0 "/Game/Materials/M_Rock_Sandstone.M_Rock_Sandstone" "None"))
  (bind _returnvalue_4 (`PrimitiveComponent.CreateDynamicMaterialInstance` (`self.Shape_Cube_DM_Core2`) 0 "/Game/Materials/M_Rock_Sandstone.M_Rock_Sandstone" "None"))
  (bind (_direction `_新規track_0`) (`Timeline|タイムライン_0`)
    (:`Update`
      (`MaterialInstanceDynamic.SetScalarParameterValue` _returnvalue_3 "Opacity" `_新規track_0`)
      (`MaterialInstanceDynamic.SetScalarParameterValue` _returnvalue_4 "Opacity" `_新規track_0`))))

(event `CrashCount`
  ;[1 1 1] NoPlayGameModeのクラッシュカウントにプラスする
  (bind _asno_play_game_mode (cast `/Game/AdditionalContents/GameMode/NoPlayGameMode` (`GameplayStatics.GetGameMode`)))
  (set `/Game/AdditionalContents/GameMode/NoPlayGameMode.CrashCount` (+ (`/Game/AdditionalContents/GameMode/NoPlayGameMode.CrashCount` _asno_play_game_mode) 1) _asno_play_game_mode))

(fn `UserConstructionScript`)