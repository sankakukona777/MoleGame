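; BP_VendingMachine_2 is a breakable vending machine that the 2D side-scroller player destroys with dig actions.
; Each Tick it checks its collision against the player's normal, up or down dig hitbox and decrements ObjectLife on overlap.
; Surviving hits trigger a left or right camera hit-stop by relative X and call an empty DamageEffect.
; The final hit increments NoPlayGameMode's CrashCount, destroys collision and sprite components, and fires BP_CharacterCamera's finish event.
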(event `self.ReceiveTick`
  (params (DeltaSeconds :type "Float (single-precision)"))
  (bind _objectlife (`self.ObjectLife`))
  (bind _digactioncollision (`self.DigActionCollision`))
  (bind _as2dside_scroller_character (cast `/Game/2DSideScrollerBP/Blueprints/2DSideScrollerCharacter` (`GameplayStatics.GetPlayerPawn` 0) :!pure true))
  (if (> (`self.ObjectLife`) 0)
    ;[1 1 1] 接触イベントをプレイヤー&掘るアクション中に限定
    (if (`/Game/2DSideScrollerBP/Blueprints/2DSideScrollerCharacter.DigActionN` _as2dside_scroller_character)
      (if (`PrimitiveComponent.IsOverlappingComponent` _digactioncollision (`/Game/2DSideScrollerBP/Blueprints/2DSideScrollerCharacter.DigActionCollision` _as2dside_scroller_character))
        ;[1 1 1] オブジェクトのライフを減らす
        (set `self.ObjectLife` (- _objectlife 1) :!label _label)
        (if (== _objectlife 0)
          (`self.CrashCount`)
          (`self.Destroy Object`)
          (bind _outactors (`GameplayStatics.GetAllActorsOfClass` "/Game/Objects/カメラ関係/BP_CharacterCamera.BP_CharacterCamera_C"))
          (`/Game/Objects/カメラ関係/BP_CharacterCamera.FinishEvent_VendingMachine` (`|GetArrayItem` _outactors))
          (elif (> _objectlife 0)
            (`self.Damage Effect`)
            (if (< (.x (`self.K2_GetActorLocation` self)) (.x (`self.K2_GetActorLocation` (`GameplayStatics.GetPlayerPawn` 0))))
              (bind _outactors_2 (`GameplayStatics.GetAllActorsOfClass` "/Game/Objects/カメラ関係/BP_CharacterCamera.BP_CharacterCamera_C"))
              (`/Game/Objects/カメラ関係/BP_CharacterCamera.HitStopEvent_VendingMachine_Right` (`|GetArrayItem` _outactors_2))
              (else
                (bind _outactors_3 (`GameplayStatics.GetAllActorsOfClass` "/Game/Objects/カメラ関係/BP_CharacterCamera.BP_CharacterCamera_C"))
                (`/Game/Objects/カメラ関係/BP_CharacterCamera.HitStopEvent_VendingMachine_Left` (`|GetArrayItem` _outactors_3)))))))
      (elif (`/Game/2DSideScrollerBP/Blueprints/2DSideScrollerCharacter.DigActionUP` _as2dside_scroller_character)
        (if (`PrimitiveComponent.IsOverlappingComponent` _digactioncollision (`/Game/2DSideScrollerBP/Blueprints/2DSideScrollerCharacter.DigActionCollisionUP` _as2dside_scroller_character))
          (goto _label))
        (elif (`/Game/2DSideScrollerBP/Blueprints/2DSideScrollerCharacter.DigActionDown` _as2dside_scroller_character)
          (if (`PrimitiveComponent.IsOverlappingComponent` _digactioncollision (`/Game/2DSideScrollerBP/Blueprints/2DSideScrollerCharacter.DigActionCollisionDOWN` _as2dside_scroller_character))
            (goto _label)))))))

(event `Damage Effect`)

(event `Destroy Object`
  (`ActorComponent.K2_DestroyComponent` (`self.DigActionCollision`))
  (`ActorComponent.K2_DestroyComponent` (`self.Sprite_01`)))

(event `CrashCount`
  ;[1 1 1] NoPlayGameModeのクラッシュカウントにプラスする
  (bind _asno_play_game_mode (cast `/Game/ゲームモード/NoPlayGameMode` (`GameplayStatics.GetGameMode`)))
  (set `/Game/ゲームモード/NoPlayGameMode.CrashCount` (+ (`/Game/ゲームモード/NoPlayGameMode.CrashCount` _asno_play_game_mode) 1) _asno_play_game_mode))

(fn `UserConstructionScript`)